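; A 2D gravity switcher actor that inverts a 2DCharacter_BP's vertical gravity as it passes through.
; While overlapped, Tick waits until the character's Z nearly matches its own, then toggles GravityUp, sets the opposite gravity direction and clears the overlap flag.
; The construction script rotates the plane mesh to match 2DGravityDirection.
; Directional switching, velocity reset and FlipFlop logic are left unconnected.
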(event Collision|EventActorBeginOverlap
  (params (OtherActor :type Actor%20Object%20Reference))
  (Variables|Default|Setoverlapping true))

(event Collision|EventActorEndOverlap
  (params (OtherActor :type Actor%20Object%20Reference))
  (Variables|Default|Setoverlapping false))

(event EventTick
  (params (DeltaSeconds :type Float%20%28single-precision%29))
  (if (Variables|Default|Getoverlapping)
    (bind _as2dcharacter_bp (Utilities|Casting|CastTo2DCharacter_BP (stale Collision|EventActorBeginOverlap OtherActor)))
    (if (Math|Float|NearlyEqual(Float) (.Z (Math|Vector|BreakVector (Transformation|GetActorLocation (stale Collision|EventActorBeginOverlap OtherActor)))) (.Z (Math|Vector|BreakVector (Transformation|GetActorLocation))) 3e+01)
      (if (Variables|/Game/Blueprints/Pawns/2DCharacter_BP.2DCharacter_BP_C|GetGravityUp _as2dcharacter_bp)
        (Variables|Default|SetGravity%20Vector "0,0.000000,-1.000000")
        (else
          (Variables|Default|SetGravity%20Vector "0, 0,1.000000")))
      (Default|SetGravityDirection _as2dcharacter_bp (Variables|Default|GetGravity%20Vector))
      (Variables|/Game/Blueprints/Pawns/2DCharacter_BP.2DCharacter_BP_C|SetGravityUp _as2dcharacter_bp (not (Variables|/Game/Blueprints/Pawns/2DCharacter_BP.2DCharacter_BP_C|GetGravityUp _as2dcharacter_bp)))
      (Variables|Default|Setoverlapping false))))

(fn ConstructionScript
  (Transformation|SetRelativeRotation (Variables|Default|GetSM_Shape_Plane) (Math|Rotator|MakeRotator 9e+01 (Utilities|Select :Index (Variables|Default|Get2DGravityDirection) :NewEnumerator0 0.0 :NewEnumerator1 1.8e+02 :NewEnumerator2 -9e+01 :NewEnumerator3 9e+01) 0.0) false false))